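; BP_Void is a fall-death volume that kills the player character when the player pawn overlaps its Box.
; Every tick it copies the player's X position while keeping its own Y and Z, so it follows along that axis.
; The first overlap plays a death sound scaled by Gameins volume settings (pitch too), then calls Die on Maincharacter_BP after a short delay.
; A W_Fail widget creation chain is left unconnected.
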(event OnComponentBeginOverlap(Box)
  (params (OverlappedComponent :type Primitive%20Component%20Object%20Reference) (OtherActor :type Actor%20Object%20Reference) (OtherComp :type Primitive%20Component%20Object%20Reference) (OtherBodyIndex :type Integer) (bFromSweep :type Boolean) (SweepResult :type Hit%20Result%20Structure%20%28by%20ref%29))
  (if (== OtherActor (Game|Player|GetPlayerPawn 0))
    (Utilities|FlowControl|DoOnce false
      (:Completed
        (bind _asgameins (Utilities|Casting|CastToGameins (Game|GetGameInstance)))
        (Audio|PlaySound2D "/Game/Sound/SF_FallenDeath.SF_FallenDeath" (* (.MasterVolume (Default|FGetSoundVolume _asgameins)) (.SFsound (Default|FGetSoundVolume _asgameins))) (* (.MasterVolume (Default|FGetSoundVolume _asgameins)) (.SFsound (Default|FGetSoundVolume _asgameins))) 0.0 0 0)
        (Utilities|FlowControl|Delay 0.5)
        (bind _asmaincharacter_bp (Utilities|Casting|CastToMaincharacter_BP (Game|Player|GetPlayerPawn 0)))
        (Default|Die _asmaincharacter_bp)))))

(event EventBeginPlay)

(event Collision|EventActorBeginOverlap
  (params (OtherActor :type Actor%20Object%20Reference)))

(event EventTick
  (params (DeltaSeconds :type Float%20%28single-precision%29))
  (bind _returnvalue (Transformation|GetActorLocation))
  (Transformation|SetActorLocation self (Math|Vector|MakeVector (.x (Transformation|GetActorLocation (Game|Player|GetPlayerPawn 0))) (.y _returnvalue) (.z _returnvalue)) false false))

(fn ConstructionScript)