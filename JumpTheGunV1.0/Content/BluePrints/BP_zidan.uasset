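; BP_zidan is an actor that plays out a fall-death sequence on the player as soon as it spawns.
; BeginPlay disables the main character's movement, switches it to Flying mode, plays the fallen-death sound, then calls Die after a one-second delay.
; Every Tick shifts both the player pawn and itself along Z by Speed, without delta-time scaling.
; Shoot-sound and fail-widget nodes are left unconnected.
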(event EventBeginPlay
  (bind _asmaincharacter_bp (Utilities|Casting|CastToMaincharacter_BP (Game|Player|GetPlayerPawn 0)))
  (Variables|/Game/BluePrints/Maincharacter_BP.Maincharacter_BP_C|SetCanMove? _asmaincharacter_bp false)
  (Pawn|Components|CharacterMovement|SetMovementMode (Variables|/Script/Engine.Character|GetCharacterMovement _asmaincharacter_bp) "MOVE_Flying" 0)
  (bind _asmaincharacter_bp_2 (Utilities|Casting|CastToMaincharacter_BP (Game|Player|GetPlayerPawn 0)))
  (Default|PlaySoundEffects _asmaincharacter_bp_2 "/Game/Sound/SF_FallenDeath.SF_FallenDeath")
  (Utilities|FlowControl|Delay 1.0)
  (bind _asmaincharacter_bp_3 (Utilities|Casting|CastToMaincharacter_BP (Game|Player|GetPlayerPawn 0)))
  (Default|Die _asmaincharacter_bp_3))

(event Collision|EventActorBeginOverlap
  (params (OtherActor :type Actor%20Object%20Reference)))

(event EventTick
  (params (DeltaSeconds :type Float%20%28single-precision%29))
  (bind _returnvalue (Game|Player|GetPlayerPawn 0))
  (bind _returnvalue_2 (Transformation|GetActorLocation))
  (bind _returnvalue_3 (Transformation|GetActorLocation _returnvalue))
  (Transformation|SetActorLocation _returnvalue (Math|Vector|MakeVector (.x _returnvalue_3) (.y _returnvalue_3) (+ (.z _returnvalue_3) (Variables|Default|GetSpeed))) false false)
  (Transformation|SetActorLocation (Math|Vector|MakeVector (.x _returnvalue_2) (.y _returnvalue_2) (+ (.z _returnvalue_2) (Variables|Default|GetSpeed))) false false))

(fn ConstructionScript)