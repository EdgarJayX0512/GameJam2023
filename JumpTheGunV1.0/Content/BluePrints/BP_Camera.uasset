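; BP_Camera is a scrolling camera that becomes the view target at BeginPlay and kills the player who falls too far behind.
; While 跟随 (follow) is true it snaps to the character; BeginPlay clears that flag after two seconds.
; It then matches player height and advances along X using walk speed and the character's capped Speed.
; Exceeding the trailing limit triggers a one-time, volume-scaled death sound, then a delayed Die call.
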(event EventBeginPlay
  (bind _asmaincharacter_bp (Utilities|Casting|CastToMaincharacter_BP (Game|Player|GetPlayerPawn 0)))
  (Variables|Default|SetAs%20Maincharacter%20BP _asmaincharacter_bp)
  (Game|Player|SetViewTargetwithBlend (Game|GetPlayerController 0) self 0.0 "VTBlend_Linear" 0.0 false)
  (Utilities|FlowControl|Delay 2.0)
  (Variables|Default|Set跟随 false))

(event Collision|EventActorBeginOverlap
  (params (OtherActor :type Actor%20Object%20Reference)))

(event EventTick
  (params (DeltaSeconds :type Float%20%28single-precision%29))
  (bind _returnvalue (Transformation|GetActorLocation))
  (bind _as_maincharacter_bp (Variables|Default|GetAs%20Maincharacter%20BP))
  (Variables|Default|GetAs%20Maincharacter%20BP
    (:then
      (if (Variables|Default|Get跟随)
        (Transformation|SetActorLocation (Transformation|GetActorLocation (Variables|Default|GetAs%20Maincharacter%20BP)) false false)
        (else
          (Transformation|SetActorLocation (Math|Vector|MakeVector (.x _returnvalue) (.y _returnvalue) (.z (Transformation|GetActorLocation (Variables|Default|GetAs%20Maincharacter%20BP)))) false false)
          (Transformation|AddActorWorldOffset (Math|Vector|MakeVector (* (Variables|/Script/Engine.CharacterMovementComponent|GetMaxWalkSpeed (Variables|/Script/Engine.Character|GetCharacterMovement _as_maincharacter_bp)) (Math|Float|Min(Float) (Variables|/Game/BluePrints/Maincharacter_BP.Maincharacter_BP_C|GetSpeed _as_maincharacter_bp) 1.0) (/ DeltaSeconds 1.0)) 0.0 0.0))
          (if (>= (- (.x (Transformation|GetActorLocation)) (.x (Transformation|GetActorLocation _as_maincharacter_bp))) 7.7e+02)
            (Utilities|FlowControl|DoOnce false
              (:Completed
                (bind _asgameins (Utilities|Casting|CastToGameins (Game|GetGameInstance)))
                (Audio|PlaySound2D "/Game/Sound/SF_Death.SF_Death" (* (.MasterVolume (Default|FGetSoundVolume _asgameins)) (.SFsound (Default|FGetSoundVolume _asgameins))) (* (.MasterVolume (Default|FGetSoundVolume _asgameins)) (.SFsound (Default|FGetSoundVolume _asgameins))) 0.0 0 0)
                (Utilities|FlowControl|Delay 0.7)
                (bind _asmaincharacter_bp (Utilities|Casting|CastToMaincharacter_BP (Game|Player|GetPlayerPawn 0)))
                (Default|Die _asmaincharacter_bp)))))))
    (:else)))

(fn ConstructionScript)