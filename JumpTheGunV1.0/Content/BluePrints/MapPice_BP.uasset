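; MapPice_BP is a weapon-shaped, self-chaining map piece that speeds up the character when its trigger box is overlapped.
; It optionally randomizes its type, then applies that type's mesh and transforms from the Weapon map.
; Barrels spawn the next piece on BeginPlay, others on overlap, then self-destroy after a delay.
; One-shot player triggers call AntMan at the Ar15 scope or fire BP_zidan with sound from Barrels.
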(event OnComponentBeginOverlap(ScopeBox)
  (params (OverlappedComponent :type Primitive%20Component%20Object%20Reference) (OtherActor :type Actor%20Object%20Reference) (OtherComp :type Primitive%20Component%20Object%20Reference) (OtherBodyIndex :type Integer) (bFromSweep :type Boolean) (SweepResult :type Hit%20Result%20Structure%20%28by%20ref%29))
  (bind _returnvalue (Game|Player|GetPlayerPawn 0))
  (if (and (Utilities|Enum|Equal(Enum) (Variables|Default|GetCurrentWeaponType) "NewEnumerator2") (== OtherActor _returnvalue))
    (Utilities|FlowControl|DoOnce false
      (:Completed
        (bind _asmaincharacter_bp (Utilities|Casting|CastToMaincharacter_BP _returnvalue))
        (Default|Ant-Man _asmaincharacter_bp)))))

(event OnComponentBeginOverlap(Box)
  (params (OverlappedComponent :type Primitive%20Component%20Object%20Reference) (OtherActor :type Actor%20Object%20Reference) (OtherComp :type Primitive%20Component%20Object%20Reference) (OtherBodyIndex :type Integer) (bFromSweep :type Boolean) (SweepResult :type Hit%20Result%20Structure%20%28by%20ref%29))
  (bind _asmaincharacter_bp (Utilities|Casting|CastToMaincharacter_BP OtherActor))
  (Variables|/Game/BluePrints/Maincharacter_BP.Maincharacter_BP_C|SetSpeed _asmaincharacter_bp (Math|Float|Clamp(Float) (+ (Variables|/Game/BluePrints/Maincharacter_BP.Maincharacter_BP_C|GetSpeed _asmaincharacter_bp) 0.05) 0.0 2.0))
  (if (not (Utilities|Enum|Equal(Enum) (Variables|Default|GetCurrentWeaponType) "NewEnumerator4"))
    (Game|SpawnActorfromClass "MapPice_BP_C" (Transformation|GetWorldTransform (Variables|Default|GetArrowEnd)) "Undefined" "MultiplyWithRoot" 0 0)
    (Utilities|FlowControl|Delay 2e+01)
    (Actor|DestroyActor)))

(event OnComponentBeginOverlap(Box1)
  (params (OverlappedComponent :type Primitive%20Component%20Object%20Reference) (OtherActor :type Actor%20Object%20Reference) (OtherComp :type Primitive%20Component%20Object%20Reference) (OtherBodyIndex :type Integer) (bFromSweep :type Boolean) (SweepResult :type Hit%20Result%20Structure%20%28by%20ref%29))
  (if (and (Utilities|Enum|Equal(Enum) (Variables|Default|GetCurrentWeaponType) "NewEnumerator4") (== OtherActor (Game|Player|GetPlayerPawn 0)))
    (Utilities|FlowControl|DoOnce false
      (:Completed
        (Game|SpawnActorfromClass "/Game/BluePrints/BP_zidan.BP_zidan_C" (Math|Conversions|ToTransform(Vector) (Transformation|GetWorldLocation (Variables|Default|GetBox1))) "AlwaysSpawn" "MultiplyWithRoot" 0 0)
        (bind _asgameins (Utilities|Casting|CastToGameins (Game|GetGameInstance)))
        (Audio|PlaySound2D "/Game/Sound/SF_Shoot.SF_Shoot" (* (.MasterVolume (Default|FGetSoundVolume _asgameins)) (.SFsound (Default|FGetSoundVolume _asgameins))) (* (.MasterVolume (Default|FGetSoundVolume _asgameins)) (.SFsound (Default|FGetSoundVolume _asgameins))) 0.0 0 0)))))

(event EventBeginPlay
  (CallFunction|FRandomWeaponType)
  (CallFunction|FInitialize)
  (if (Utilities|Enum|Equal(Enum) (Variables|Default|GetCurrentWeaponType) "NewEnumerator4")
    (Game|SpawnActorfromClass "MapPice_BP_C" (Math|Conversions|ToTransform(Vector) (CallFunction|FGetArrowEndLocation)) "Undefined" "MultiplyWithRoot" 0 0)
    (Utilities|FlowControl|Delay 2e+01)
    (Actor|DestroyActor)))

(fn ConstructionScript
  (CallFunction|FInitialize))

(fn FInitialize
  (bind _currentweapontype (Variables|Default|GetCurrentWeaponType))
  (bind _weapon (Variables|Default|Getweapon))
  (bind _value (Utilities|Map|Find _weapon _currentweapontype))
  (bind (_arrowstart_transform _arrowend_transform _box_transform _weapon_transform _actorscaling) (Utilities|Struct|BreakE_WeaponData _value))
  (Transformation|SetRelativeTransform (Variables|Default|GetArrowStart) _arrowstart_transform false false)
  (Transformation|SetRelativeTransform (Variables|Default|GetArrowEnd) _arrowend_transform false false)
  (Transformation|SetRelativeTransform (Variables|Default|GetBox) _box_transform false false)
  (Transformation|SetRelativeTransform (Variables|Default|GetWeaponMesh) _weapon_transform false false)
  (Transformation|SetActorRelativeScale3D _actorscaling)
  (Components|StaticMesh|SetStaticMesh (Variables|Default|GetWeaponMesh) (Utilities|Select :Index (Variables|Default|GetCurrentWeaponType) :NewEnumerator5 0 :NewEnumerator0 "/Game/Assets/3D_Assets/am.am" :NewEnumerator1 "/Game/Assets/3D_Assets/apex.apex" :NewEnumerator2 "/Game/Assets/3D_Assets/ar15.ar15" :NewEnumerator3 "/Game/Assets/3D_Assets/Bow.Bow" :NewEnumerator4 "/Game/Assets/3D_Assets/123.123")))

(fn FRandomWeaponType
  (if (Variables|Default|GetIsRanderWeapon?)
    (bind _keys (Utilities|Map|Keys (Variables|Default|Getweapon) :!label _label))
    (if (Utilities|Enum|NotEqual(Enum) (.OutItem (Utilities|Array|Random _keys)) (Variables|Default|GetCurrentWeaponType))
      (Variables|Default|SetCurrentWeaponType (.OutItem (Utilities|Array|Random _keys)))
      (return)
      (else
        (goto _label)))))

(fn FGetArrowEndLocation
  (return (Transformation|GetWorldLocation (Variables|Default|GetArrowEnd))))