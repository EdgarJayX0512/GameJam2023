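; Gameins, apparently a Game Instance going by its name, stores the game's master, sound effect and background volume levels.
; The Updata_Volume event saves the three incoming values and then calls the EDUpdataSoundVolume event dispatcher to broadcast the change.
; FGetSoundVolume returns the stored levels to callers.
; A debug print of the values is left unconnected.
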(event Custom|Updata_Volume
  (params (MasterVolume :type Float%20%28double-precision%29) (SFsound :type Float%20%28double-precision%29) (BGsound :type Float%20%28double-precision%29))
  (Variables|Default|SetMasterVolume MasterVolume)
  (Variables|Default|SetSFsound SFsound)
  (Variables|Default|SetBGsound BGsound)
  (Default|CallEDUpdataSoundVolume))

(fn FGetSoundVolume
  (return (Variables|Default|GetMasterVolume) (Variables|Default|GetSFsound) (Variables|Default|GetBGsound)))