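; BP_BackgroundMusic is an actor that keeps the background music volume in line with the player's sound settings.
; On BeginPlay it casts to the Gameins game instance, binds to its sound-volume update dispatcher and triggers a volume update.
; The update handler sets the Audio component's volume multiplier to master volume times background volume and prints the result.
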(event Custom|Updata_SoundVolume
  (bind _as_gameins (Variables|Default|GetAs%20Gameins))
  (bind (_mastervolume _sfsound _bgsound) (Default|FGetSoundVolume _as_gameins))
  (bind _returnvalue (* _mastervolume _bgsound))
  (Audio|Components|Audio|SetVolumeMultiplier (Variables|Default|GetAudio) _returnvalue :!class /Script/Engine.AudioComponent)
  (Development|PrintString (Utilities|String|ToString(Float) _returnvalue)))

(event Collision|EventActorBeginOverlap
  (params (OtherActor :type Actor%20Object%20Reference)))

(event EventTick
  (params (DeltaSeconds :type Float%20%28single-precision%29)))

(event EventBeginPlay
  (bind _asgameins (Utilities|Casting|CastToGameins (Game|GetGameInstance)))
  (bind _output_get (Variables|Default|SetAs%20Gameins _asgameins))
  (EventDispatchers|BindEventtoEDUpdataSoundVolume _output_get (EventDispatchers|CreateEvent :!event Custom|Updata_SoundVolume))
  (CallFunction|UpdataSoundVolume))

(fn ConstructionScript)