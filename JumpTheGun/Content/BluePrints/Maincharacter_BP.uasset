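; Player character Blueprint that runs automatically along world +X and handles jumping and pausing.
; Tick feeds Speed into movement input as its scale and prints that value to screen.
; JumpAction triggers Jump and holds IsJumping true for a fixed short delay, independent of landing.
; IA_Pause toggles a newly created pause menu widget along with game pause, input mode and mouse cursor.
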(event Input|EnhancedActionEvents|EnhancedInputActionIA_Pause
  (params (ActionValue :type Boolean) (ElapsedSeconds :type Float%20%28double-precision%29) (TriggeredSeconds :type Float%20%28double-precision%29) (InputAction :type Input%20Action%20Object%20Reference :default "/Game/Input/IA_Pause.IA_Pause"))
  (bind _returnvalue (Game|GetPlayerController 0))
  (:Started
    (if (not (Variables|Default|GetIsPausemenuOpened?))
      (Variables|Default|SetIsPausemenuOpened? true)
      (UserInterface|CreateWidget "/Game/UI/Pausemenu_BP.Pausemenu_BP_C" _returnvalue)
      (bind _output_get (Variables|Default|SetPause%20Menu%20Widget (Variables|Default|GetPause%20Menu%20Widget)))
      (UserInterface|Viewport|AddtoViewport _output_get 0)
      (Input|SetInputModeGameandUI _returnvalue (Variables|Default|GetPause%20Menu%20Widget) "DoNotLock" true false)
      (Variables|/Script/Engine.PlayerController|SetbShowMouseCursor (Game|GetPlayerController 0) true)
      (Game|SetGamePaused true)
      (else
        (Variables|Default|SetIsPausemenuOpened? false)
        (Widget|RemovefromParent (Variables|Default|GetPause%20Menu%20Widget))
        (Game|SetGamePaused false)
        (Input|SetInputModeGameOnly _returnvalue false)
        (Variables|/Script/Engine.PlayerController|SetbShowMouseCursor (Game|GetPlayerController 0) false)))))

(event EventBeginPlay)

(event Collision|EventActorBeginOverlap
  (params (OtherActor :type Actor%20Object%20Reference)))

(event EventTick
  (params (DeltaSeconds :type Float%20%28single-precision%29))
  (Pawn|Input|AddMovementInput "1.000000,0.000000,0.000000" (Variables|Default|GetSpeed) false)
  (Development|PrintString (Utilities|String|ToString(Float) (Variables|Default|GetSpeed))))

(event Input|ActionEvents|InputActionJumpAction
  (params (Key :type Key%20Structure :default "None"))
  (:Pressed
    (Character|Jump)
    (Variables|Default|SetIsJumping true)
    (Utilities|FlowControl|Delay 0.6)
    (Variables|Default|SetIsJumping false)))

(fn ConstructionScript)